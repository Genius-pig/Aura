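; Gameplay ability for an enemy ranged attack that fires a projectile at the avatar's combat target.
; On activation it turns the avatar toward the target and plays a random tagged montage from the avatar's attack montages.
; A one-shot gameplay event matching the montage's attack tag triggers the projectile, aimed at the target's re-queried location with a pitch override.
; The ability ends when the montage completes, is interrupted or is cancelled.
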(event Ability|EventActivateAbility
  (bind _returnvalue (Ability|GetAvatarActorfromActorInfo))
  (bind _returnvalue_2 (Class|EnemyInterface|GetCombatTarget(Message) _returnvalue))
  (bind _ascombat_interface (Utilities|Casting|CastToCombatInterface _returnvalue))
  (Class|CombatInterface|SetFacingTarget _ascombat_interface (Transformation|GetActorLocation _returnvalue_2))
  (bind _returnvalue_3 (Class|CombatInterface|GetAttackMontage(Message) (Ability|GetAvatarActorfromActorInfo)))
  (bind _output_get (Variables|Default|SetTaggedMontage (Class|AuraDamageGameplayAbility|GetRandomTaggedMontagefromArray _returnvalue_3)))
  (Variables|Default|SetAttack%20Tag (.AttackTag (Utilities|Struct|BreakTaggedMontage _output_get)))
  (|PlayMontageandWaitProxy "None" (.Montage (Utilities|Struct|BreakTaggedMontage _output_get)) 1.0 "None" false 1.0 0.0
    (:then
      (Ability|Tasks|WaitGameplayEvent (Variables|Default|GetAttack%20Tag) 0 true
        (:EventReceived
          (bind _returnvalue_4 (Class|EnemyInterface|GetCombatTarget(Message) (Ability|GetAvatarActorfromActorInfo)))
          (Class|AuraProjectileSpell|SpawnProjectile (Transformation|GetActorLocation _returnvalue_4) (Variables|Default|GetAttack%20Tag) true 2.0))))
    (:OnCompleted
      (Ability|EndAbility :!label _label))
    (:OnInterrupted
      (goto _label))
    (:OnCancelled
      (goto _label))))

(event Ability|EventOnEndAbility
  (params (bWasCancelled :type Boolean)))