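; GA_FireBolt is the Fire Bolt gameplay ability that casts homing-capable fire projectiles at whatever is under the mouse cursor.
; After committing, it reads target data from the cursor, turns the avatar toward the hit location and plays the cast montage.
; A montage gameplay event triggers SpawnProjectiles from the weapon socket, passing the hit actor as homing target.
; The ability ends when the montage completes, is interrupted or is cancelled.
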(event Ability|EventActivateAbility
  (Ability|CommitAbility)
  (bind _data (|GetTargetDataUnderMouse)
    (:ValidData
      (Variables|Default|SetLocation (.Location (Collision|BreakHitResult (Ability|TargetData|GetHitResultfromTargetData _data))))
      (Variables|Default|SetHit%20Actor (.HitActor (Collision|BreakHitResult (Ability|TargetData|GetHitResultfromTargetData _data))))
      (Class|CombatInterface|SetFacingTarget(Message) (Ability|GetAvatarActorfromActorInfo) (Variables|Default|GetLocation))
      (|PlayMontageandWaitProxy "None" "/Game/Assets/Characters/Aura/Animations/Abilities/AM_Cast_FireBolt.AM_Cast_FireBolt" 1.0 "None" false 1.0 0.0
        (:then
          (Ability|Tasks|WaitGameplayEvent "(TagName=\"Event.Montage.FireBolt\")" 0
            (:EventReceived
              (Class|AuraFireBolt|SpawnProjectiles (Variables|Default|GetLocation) (GameplayTags|MakeLiteralGameplayTag "(TagName=\"Attack.Weapon\")") false 0.0 (Variables|Default|GetHit%20Actor)))))
        (:OnCompleted
          (Ability|EndAbility :!label _label))
        (:OnInterrupted
          (goto _label))
        (:OnCancelled
          (goto _label))))))

(event Ability|EventOnEndAbility
  (params (bWasCancelled :type Boolean)))