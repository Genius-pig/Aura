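; Arcane Shards gameplay ability that shows a magic circle, then spawns shard cues at the targeted point when input is released.
; On release it gets target data under the mouse, builds randomly rotated ground points via a spawned BP_PointCollection, faces the target and plays the cast montage.
; The montage event hides the circle and starts a looping timer that fires one gameplay cue and debug sphere per point, then destroys the collection and ends.
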(event Custom|SpawnShard
  (if (< (Variables|Default|GetCount) (Variables|Default|GetNumPoints))
    (bind _output_get (Variables|Default|SetShardSpawnLocation (Transformation|GetWorldLocation (Utilities|Array|Get(acopy) (Variables|Default|GetGroundPoints) (Variables|Default|GetCount)))))
    (Rendering|Debug|DrawDebugSphere _output_get 1e+01 12 "(R=1.000000,G=0.000000,B=0.146509,A=1.000000)" 1e+01)
    (Math|Integer|IncrementInt (Variables|Default|GetCount)
      (:%20%20
        (Class|GameplayAbility|ExecuteGameplayCuewithParams "(TagName=\"GameplayCue.ArcaneShards\")" (Ability|GameplayCue|MakeGameplayCueParameters :Location (Variables|Default|GetShardSpawnLocation)))))
    (else
      (Utilities|Time|ClearandInvalidateTimerbyHandle (Variables|Default|GetShardSpawnTimer))
      (Actor|DestroyActor (Variables|Default|GetPointCollection))
      (Ability|EndAbility))))

(event Ability|EventActivateAbility
  (Utilities|FlowControl|Sequence
    (:then_0
      (Class|PlayerInterface|ShowMagicCircle(Message) (Ability|GetAvatarActorfromActorInfo) 0))
    (:then_1
      (Ability|Tasks|WaitInputRelease false
        (:OnRelease
          (bind _data (|GetTargetDataUnderMouse)
            (:ValidData
              (Variables|Default|SetMouseHitLocation (.ImpactPoint (Collision|BreakHitResult (Ability|TargetData|GetHitResultfromTargetData _data))))
              (bind _returnvalue (Game|SpawnActorfromClass "/Game/Blueprints/AbilitySystem/Aura/Abilities/Arcane/ArcaneShards/BP_PointCollection.BP_PointCollection_C" (Math|Transform|MakeTransform (Variables|Default|GetMouseHitLocation) "0, 0, 0" "1.000000,1.000000,1.000000") "AlwaysSpawn" "MultiplyWithRoot" 0 0))
              (Variables|Default|SetPointCollection _returnvalue)
              (Variables|Default|SetGroundPoints (Class|PointCollection|GetGroundPoints (Variables|Default|GetPointCollection) (Variables|Default|GetMouseHitLocation) (Variables|Default|GetNumPoints) (Math|Random|RandomFloatinRange 0.0 3.6e+02)))
              (Class|CombatInterface|SetFacingTarget(Message) (Ability|GetAvatarActorfromActorInfo) (Variables|Default|GetMouseHitLocation))
              (|PlayMontageandWaitProxy "None" "/Game/Assets/Characters/Aura/Animations/Abilities/AM_Cast_ArcaneShards.AM_Cast_ArcaneShards" 1.0 "None" true 1.0 0.0
                (:then
                  (Ability|Tasks|WaitGameplayEvent "(TagName=\"Event.Montage.ArcaneShards\")" 0 true
                    (:EventReceived
                      (bind _returnvalue_2 (Utilities|Time|SetTimerbyEvent (delegate Custom|SpawnShard) (Variables|Default|GetShardSpawnDeltaTime) true))
                      (Variables|Default|SetShardSpawnTimer _returnvalue_2)
                      (CallFunction|SpawnShard)
                      (Class|PlayerInterface|HideMagicCircle(Message) (Ability|GetAvatarActorfromActorInfo)))))))))))))

(event Ability|EventOnEndAbility
  (params (bWasCancelled :type Boolean)))