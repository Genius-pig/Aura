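; GA_FireBolt is a gameplay ability that casts a fire bolt projectile toward the point under the mouse.
; On activation it takes the hit location from mouse target data, turns the avatar to face it through CombatInterface and plays the cast montage.
; A Montage.Attack.Weapon gameplay event during the montage spawns the projectile at that target, and the ability ends when the montage completes, blends out, is interrupted or is cancelled.
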(event Ability|EventActivateAbility
  (bind _data (|GetTargetDataUnderMouse)
    (:ValidData
      (Variables|Default|SetLocation (.Location (Collision|BreakHitResult (Ability|TargetData|GetHitResultfromTargetData _data))))
      (bind _ascombat_interface (Utilities|Casting|CastToCombatInterface (Ability|GetAvatarActorfromActorInfo)))
      (Class|CombatInterface|SetFacingTarget _ascombat_interface (Variables|Default|GetLocation))
      (|PlayMontageandWaitProxy "None" "/Game/Assets/Characters/Aura/Animations/Abilities/AM_Cast_FireBolt.AM_Cast_FireBolt" 1.0 "None" true 1.0 0.0
        (:then
          (Ability|Tasks|WaitGameplayEvent "(TagName=\"Montage.Attack.Weapon\")" 0
            (:EventReceived
              (Class|AuraProjectileSpell|SpawnProjectile (Variables|Default|GetLocation)))))
        (:OnCompleted
          (Ability|EndAbility :!label _label))
        (:OnBlendOut
          (goto _label))
        (:OnInterrupted
          (goto _label))
        (:OnCancelled
          (goto _label))))))

(event Ability|EventOnEndAbility
  (params (bWasCancelled :type Boolean)))